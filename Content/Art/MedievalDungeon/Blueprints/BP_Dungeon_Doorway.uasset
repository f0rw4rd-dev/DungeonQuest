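; Dungeon doorway Blueprint that swings its left door mesh between yaw-closed and open positions.
; On BeginPlay it snaps the door open unless the Closed flag is set.
; OpenDoor and CloseDoor update Closed and lerp the yaw through timelines with swapped names: opening uses CloseDoorTimeline, closing uses OpenDoorTimeline.
; Both timelines use Play rather than PlayFromStart, so neither rewinds before a repeat call.
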(event `self.ReceiveBeginPlay`
  ;[0 0 0] Begin play
  (if (not (`self.bClosed`))
    (`self.OpenDoorFast`)))

(event `OpenDoorFast`
  ;[0 0 0] Open door fast
  (set `self.bClosed` false)
  (`SceneComponent.K2_SetRelativeRotation` (`self.SM_DoorWay_Large_Door_Left`) (`KismetMathLibrary.MakeRotator` 0.0 0.0 70.0) false false))

(event `OpenDoor`
  ;[0 0 0] Open door
  (set `self.bClosed` false)
  (bind (_direction _alpha) (`Timeline|CloseDoorTimeline`)
    (:`Update`
      (`SceneComponent.K2_SetRelativeRotation` (`self.SM_DoorWay_Large_Door_Left`) (`KismetMathLibrary.MakeRotator` 0.0 0.0 (`KismetMathLibrary.Lerp` 0.0 70.0 _alpha)) false false))))

(event `CloseDoor`
  ;[0 0 0] Close door
  (set `self.bClosed` true)
  (bind (_direction _alpha) (`Timeline|OpenDoorTimeline`)
    (:`Update`
      (`SceneComponent.K2_SetRelativeRotation` (`self.SM_DoorWay_Large_Door_Left`) (`KismetMathLibrary.MakeRotator` 0.0 0.0 (`KismetMathLibrary.Lerp` 70.0 0.0 _alpha)) false false))))

(fn `UserConstructionScript`)