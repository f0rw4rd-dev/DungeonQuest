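; BP_Room01 is a procedural dungeon room with an entry, same- and higher-difficulty exits, spike traps and bonuses.
; On BeginPlay it caches doorway transforms and assigns each moving spike trap its spline path.
; It gathers tagged child actors, then calls helpers that randomly cull traps and pills and remove health recovery based on difficulty.
; The first overlap of the entered-room trigger closes the entry door and generates the next rooms.
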(event `self.ReceiveBeginPlay`
  (bind _bp_dungeon_doorway_entry (`self.BP_Dungeon_Doorway_Entry`))
  (bind _bp_dungeon_doorway_higherdifficulty (`self.BP_Dungeon_Doorway_HigherDifficulty`))
  (bind _returnvalue (`SceneComponent.K2_GetComponentToWorld` (`self.BP_Dungeon_Doorway_SameDifficulty`)))
  ;[0 0 0] Begin play
  (`parent.ReceiveBeginPlay`)
  (set `self.EntryDoorRelativeTransform` (`SceneComponent.GetRelativeTransform` _bp_dungeon_doorway_entry))
  (set `self.EntryDoorWorldTransform` (`SceneComponent.K2_GetComponentToWorld` _bp_dungeon_doorway_entry))
  (set `self.HigherDifficultyExitDoorRelativeTransform` (`SceneComponent.GetRelativeTransform` _bp_dungeon_doorway_higherdifficulty))
  (set `self.HigherDifficultyExitDoorWorldTransform` (`SceneComponent.K2_GetComponentToWorld` _bp_dungeon_doorway_higherdifficulty))
  (set `self.SameDifficultyExitDoorRelativeTransform` _returnvalue)
  (set `self.SameDifficultyExitDoorWorldTransform` _returnvalue)
  (bind _output_get (set `self.MovingSpikeTraps` (`|MakeMap` (`self.BP_MovingSpikeTrap1`) (`self.SC_TrapPath1`) (`self.BP_MovingSpikeTrap2`) (`self.SC_TrapPath2`) (`self.BP_MovingSpikeTrap3`) (`self.SC_TrapPath3`) (`self.BP_MovingSpikeTrap4`) (`self.SC_TrapPath4`) (`self.BP_MovingSpikeTrap5`) (`self.SC_TrapPath5`))))
  (bind _keys (`BlueprintMapLibrary.Map_Keys` _output_get))
  (for _array_element _keys
    (bind _asbp_moving_spike_trap (cast `/Game/Core/Systems/Traps/Dynamic/BP_MovingSpikeTrap` (`ChildActorComponent.ChildActor` _array_element)))
    (set `/Game/Core/Systems/Traps/Dynamic/BP_MovingSpikeTrap.Spline` (`BlueprintMapLibrary.Map_Find` (`self.MovingSpikeTraps`) _array_element) _asbp_moving_spike_trap))
  (set `self.SpikeTraps` (`self.GetComponentsByTag` "/Script/Engine.ChildActorComponent" "SpikeTrap"))
  (set `self.PillBonuses` (`self.GetComponentsByTag` "/Script/Engine.ChildActorComponent" "PillBonus"))
  (set `self.HealthRecovery` (`self.BP_Bonus_HealthRecovery`))
  (`self.DestroyRandomSpikeTraps`)
  (`self.DestroyRandomMovingSpikeTraps`)
  (`self.DestroyRandomPillBonuses`)
  (`self.DestroyBonusHealthRecoveryDependingOnDifficulty`))

(event `self.SM_TB_EnteredRoom.OnComponentBeginOverlap`
  (params (OverlappedComponent :type "PrimitiveComponent Object Reference") (OtherActor :type "Actor Object Reference") (OtherComp :type "PrimitiveComponent Object Reference") (OtherBodyIndex :type Integer) (bFromSweep :type Boolean) (SweepResult :type "HitResult Structure (by ref)"))
  ;[0 0 0] Close entry door
  (`/Engine/EditorBlueprintResources/StandardMacros.DoOnce` false
    (:`Completed`
      (bind _asbp_dungeon_doorway (cast `/Game/Art/MedievalDungeon/Blueprints/BP_Dungeon_Doorway` (`ChildActorComponent.ChildActor` (`self.BP_Dungeon_Doorway_Entry`))))
      (`/Game/Art/MedievalDungeon/Blueprints/BP_Dungeon_Doorway.CloseDoor` _asbp_dungeon_doorway)
      (`self.GenerateNextRooms`))))

(fn `UserConstructionScript`)