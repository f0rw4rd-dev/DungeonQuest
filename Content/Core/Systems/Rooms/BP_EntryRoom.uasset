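; Entry room actor that seeds a run of linked rooms by spawning the first one on BeginPlay.
; It randomly picks one of two room classes and builds its RoomInfo from the "Normal" difficulty row, with fallback defaults and a random room limit.
; The room spawns at the entry's location with a fixed flipped rotation and records the entry in its PreviousRooms.
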(event `self.ReceiveBeginPlay`
  (bind (_returnvalue_location _returnvalue_rotation _returnvalue_scale) (`KismetMathLibrary.BreakTransform` (`self.GetTransform`)))
  (bind _returnvalue (`KismetMathLibrary.RandomIntegerInRange` 6 10))
  ;[0 0 0] Begin Play
  (switch `int` (`KismetMathLibrary.RandomIntegerInRange` 0 1)
    (:`Default`
      (set `self.Room` "/Game/Core/Systems/Rooms/BP_Room02.BP_Room02_C" :!label _label))
    (:`0`
      (set `self.Room` "/Game/Core/Systems/Rooms/BP_Room01.BP_Room01_C"))
    (:`1`
      (goto _label)))
  (bind _returnvalue_2 (`|GetDataTableRow` "/Game/Core/Systems/Difficulty/DT_GameDifficulties.DT_GameDifficulties" "Normal")
    (:`then`
      (set `self.RoomInfo` (make `/Game/Core/Systems/Rooms/F_RoomInfo` 1 _returnvalue false (break `/Game/Core/Systems/Difficulty/F_GameDifficulty` _returnvalue_2) (`.StartTrapSpeed_18_1CE4E5994CA5395A0B7299BABF0AA1FB` (break `/Game/Core/Systems/Difficulty/F_GameDifficulty` _returnvalue_2)) (`.StartBonusDuration_19_A1834D7C40A0B809891EAEBA56AE3AC2` (break `/Game/Core/Systems/Difficulty/F_GameDifficulty` _returnvalue_2)))))
    (:`RowNotFound`
      (set `self.RoomInfo` (make `/Game/Core/Systems/Rooms/F_RoomInfo` 1 _returnvalue false 0.5 1.0 5.0))))
  (bind _returnvalue_3 (`|SpawnActorFromClass` :`Class` (`self.Room`) :`SpawnTransform` (`KismetMathLibrary.MakeTransform` _returnvalue_location (struct :`Yaw` 180.0) _returnvalue_scale) :`CollisionHandlingOverride` "Undefined" :`TransformScaleMethod` "MultiplyWithRoot" :`RoomInfo` (`self.RoomInfo`) :`Instigator` null))
  (`BlueprintSetLibrary.Set_Add` (`/Game/Core/Systems/Rooms/BP_Room.PreviousRooms` _returnvalue_3) self))

(fn `UserConstructionScript`)