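; Dungeon room actor that builds a branching run one step ahead of the player and randomizes its own content.
; On player entry it shuts the entry door, spawns higher- and same-difficulty successor rooms at their doors, ending in a last room, and destroys previous rooms.
; RoomInfo passes difficulty forward, scaled by a data table for the harder branch.
; Tagged child-actor traps and pickups are pruned by difficulty-weighted chance, with health recovery kept only on harder branches.
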(event `self.ReceiveBeginPlay`
  ;[0 0 0] Begin Play
  (`BlueprintSetLibrary.Set_Add` (`self.PreviousRooms`) self)
  (set `self.SpikeTraps` (`self.GetComponentsByTag` "/Script/Engine.ChildActorComponent" "SpikeTrap"))
  (set `self.PillBonuses` (`self.GetComponentsByTag` "/Script/Engine.ChildActorComponent" "PillBonus"))
  (set `self.HealthRecovery` (`self.FindComponentByTag` "/Script/Engine.ChildActorComponent" "HealthRecovery"))
  (set `self.EntryDoor` (`self.FindComponentByTag` "/Script/Engine.ChildActorComponent" "EntryDoor"))
  (set `self.HigherDifficultyDoor` (`self.FindComponentByTag` "/Script/Engine.ChildActorComponent" "HigherDifficultyDoor"))
  (set `self.SameDifficultyDoor` (`self.FindComponentByTag` "/Script/Engine.ChildActorComponent" "SameDifficultyDoor")))

(event `On Player Enter Room`
  (params (OtherActor :type "Actor Object Reference"))
  (bind (_roominfo_roomnumber _roominfo_maxrooms) (break `/Game/Core/Systems/Rooms/F_RoomInfo` (`self.RoomInfo`)))
  ;[0 0 0] Player Enter Room
  (bind _asbp_cabbage_seller_character (cast `/Game/Core/Characters/CabbageSeller/BP_CabbageSeller_Character` OtherActor))
  (`/Engine/EditorBlueprintResources/StandardMacros.DoOnce` false
    (:`Completed`
      (set `/Game/Core/Characters/CabbageSeller/BP_CabbageSeller_Character.bIgnoreStaticTraps` false _asbp_cabbage_seller_character)
      (set `CharacterMovementComponent.MaxWalkSpeed` 500.0 (`Character.CharacterMovement` _asbp_cabbage_seller_character))
      (bind _asbp_dungeon_doorway (cast `/Game/Art/MedievalDungeon/Blueprints/BP_Dungeon_Doorway` (`ChildActorComponent.ChildActor` (`self.EntryDoor`))))
      (`/Game/Art/MedievalDungeon/Blueprints/BP_Dungeon_Doorway.CloseDoor` _asbp_dungeon_doorway)
      (if (< _roominfo_roomnumber _roominfo_maxrooms)
        (`self.GenerateNextRooms`)))))

(fn `DestroyBonusHealthRecoveryDependingOnDifficulty`
  (bind (_roominfo_roomnumber _roominfo_maxrooms _roominfo_bhigherdifficulty) (break `/Game/Core/Systems/Rooms/F_RoomInfo` (`self.RoomInfo`)))
  (if (not _roominfo_bhigherdifficulty)
    (`/Engine/EditorBlueprintResources/StandardMacros.IsValid` (`self.HealthRecovery`)
      (:`Is Valid`
        (`ActorComponent.K2_DestroyComponent` (`self.HealthRecovery`))))))

(fn `DestroyPreviousRooms`
  (bind _result (`BlueprintSetLibrary.Set_ToArray` (`self.PreviousRooms`)))
  (for _array_element _result
    (`BlueprintSetLibrary.Set_Remove` (`self.PreviousRooms`) _array_element)
    (`/Engine/EditorBlueprintResources/StandardMacros.IsValid` _array_element
      (:`Is Valid`
        (if (!= self _array_element)
          (`self.K2_DestroyActor` _array_element))))))

(fn `DestroyRandomMovingSpikeTraps`
  (bind (_roominfo_roomnumber _roominfo_maxrooms _roominfo_bhigherdifficulty _roominfo_difficultyfactor) (break `/Game/Core/Systems/Rooms/F_RoomInfo` (`self.RoomInfo`)))
  (bind _keys (`BlueprintMapLibrary.Map_Keys` (`self.MovingSpikeTraps`)))
  (for _array_element _keys
    (if (`KismetMathLibrary.RandomBoolWithWeight` _roominfo_difficultyfactor)
      (`ActorComponent.K2_DestroyComponent` (`BlueprintMapLibrary.Map_Find` (`self.MovingSpikeTraps`) _array_element))
      (`ActorComponent.K2_DestroyComponent` _array_element))))

(fn `DestroyRandomPillBonuses`
  (bind (_roominfo_roomnumber _roominfo_maxrooms _roominfo_bhigherdifficulty _roominfo_difficultyfactor) (break `/Game/Core/Systems/Rooms/F_RoomInfo` (`self.RoomInfo`)))
  (for _array_element (`self.PillBonuses`)
    (`/Engine/EditorBlueprintResources/StandardMacros.IsValid` _array_element
      (:`Is Valid`
        (if (`KismetMathLibrary.RandomBoolWithWeight` (- 1.0 _roominfo_difficultyfactor))
          (`ActorComponent.K2_DestroyComponent` _array_element))))))

(fn `DestroyRandomSpikeTraps`
  (bind (_roominfo_roomnumber _roominfo_maxrooms _roominfo_bhigherdifficulty _roominfo_difficultyfactor) (break `/Game/Core/Systems/Rooms/F_RoomInfo` (`self.RoomInfo`)))
  (for _array_element (`self.SpikeTraps`)
    (`/Engine/EditorBlueprintResources/StandardMacros.IsValid` _array_element
      (:`Is Valid`
        (if (`KismetMathLibrary.RandomBoolWithWeight` _roominfo_difficultyfactor)
          (`ActorComponent.K2_DestroyComponent` _array_element))))))

(fn `GenerateNextRooms`
  (locals (SameDifficultyRoomInfo :type "/Game/Core/Systems/Rooms/F_RoomInfo Structure") (HigherDifficultyRoomInfo :type "/Game/Core/Systems/Rooms/F_RoomInfo Structure") (Room :type "/Game/Core/Systems/Rooms/BP_Room Class Reference") (ChangeDifficultyFactor :type "Float (double-precision)" :default 0.8) (ChangeTrapSpeed :type "Float (double-precision)" :default 1.2) (ChangeBonusDuration :type "Float (double-precision)" :default 0.8))
  (bind (_roominfo_roomnumber _roominfo_maxrooms _roominfo_bhigherdifficulty _roominfo_difficultyfactor _roominfo_trapspeed _roominfo_bonusduration) (break `/Game/Core/Systems/Rooms/F_RoomInfo` (`self.RoomInfo`)))
  (bind (_roominfo_roomnumber_2 _roominfo_maxrooms_2 _roominfo_bhigherdifficulty_2 _roominfo_difficultyfactor_2 _roominfo_trapspeed_2 _roominfo_bonusduration_2) (break `/Game/Core/Systems/Rooms/F_RoomInfo` (`self.RoomInfo`)))
  (bind (_roominfo_roomnumber_3 _roominfo_maxrooms_3) (break `/Game/Core/Systems/Rooms/F_RoomInfo` (`self.RoomInfo`)))
  (bind _returnvalue (`|GetDataTableRow` "/Game/Core/Systems/Difficulty/DT_GameDifficulties.DT_GameDifficulties" "Normal")
    (:`then`
      (set `local.ChangeDifficultyFactor` (`.ChangeDifficultyFactor_26_DB6458FF47088ECC94A700B3CFD274B9` (break `/Game/Core/Systems/Difficulty/F_GameDifficulty` _returnvalue)))
      (set `local.ChangeTrapSpeed` (`.ChangeTrapSpeed_27_999E62D6438FDA4CF58FB7A873C4533A` (break `/Game/Core/Systems/Difficulty/F_GameDifficulty` _returnvalue)))
      (set `local.ChangeBonusDuration` (`.ChangeBonusDuration_28_D2DD4ECE413E97DCBED0B4A7104C7544` (break `/Game/Core/Systems/Difficulty/F_GameDifficulty` _returnvalue))))
    (:`RowNotFound`
      _))
  (set `local.HigherDifficultyRoomInfo` (make `/Game/Core/Systems/Rooms/F_RoomInfo` (+ _roominfo_roomnumber 1) _roominfo_maxrooms true (* (`local.ChangeDifficultyFactor`) _roominfo_difficultyfactor) (* (`local.ChangeTrapSpeed`) _roominfo_trapspeed) (* _roominfo_bonusduration (`local.ChangeBonusDuration`))))
  (set `local.SameDifficultyRoomInfo` (make `/Game/Core/Systems/Rooms/F_RoomInfo` (+ _roominfo_roomnumber_2 1) _roominfo_maxrooms_2 false _roominfo_difficultyfactor_2 _roominfo_trapspeed_2 _roominfo_bonusduration_2))
  (if (< _roominfo_roomnumber_3 (- _roominfo_maxrooms_3 1))
    (switch `int` (`KismetMathLibrary.RandomIntegerInRange` 0 1)
      (:`Default`
        (set `local.Room` "/Game/Core/Systems/Rooms/BP_Room02.BP_Room02_C" :!label _label))
      (:`0`
        (set `local.Room` "/Game/Core/Systems/Rooms/BP_Room01.BP_Room01_C"))
      (:`1`
        (goto _label)))
    (else
      (set `local.Room` "/Game/Core/Systems/Rooms/BP_LastRoom01.BP_LastRoom01_C")))
  (bind _returnvalue_2 (`|SpawnActorFromClass` (`local.Room`) (`SceneComponent.K2_GetComponentToWorld` (`self.HigherDifficultyDoor`)) "Undefined" "MultiplyWithRoot" (`self.GetOwner`) (`local.HigherDifficultyRoomInfo`) (`self.PreviousRooms`) null))
  (bind _returnvalue_3 (`|SpawnActorFromClass` (`local.Room`) (`SceneComponent.K2_GetComponentToWorld` (`self.SameDifficultyDoor`)) "Undefined" "MultiplyWithRoot" (`self.GetOwner`) (`local.SameDifficultyRoomInfo`) (`self.PreviousRooms`) null))
  (bind _array (`|MakeArray` _returnvalue_3 _returnvalue_2 :!type "Actor Object Reference"))
  (`BlueprintSetLibrary.Set_AddItems` (`/Game/Core/Systems/Rooms/BP_Room.PreviousRooms` _returnvalue_3) _array)
  (`BlueprintSetLibrary.Set_AddItems` (`/Game/Core/Systems/Rooms/BP_Room.PreviousRooms` _returnvalue_2) _array)
  (`self.DestroyPreviousRooms`))

(fn `RandomizeContent`
  (`self.DestroyRandomSpikeTraps`)
  (`self.DestroyRandomMovingSpikeTraps`)
  (`self.DestroyRandomPillBonuses`)
  (`self.DestroyBonusHealthRecoveryDependingOnDifficulty`))

(fn `RunMovingSpikeTraps`
  (bind _keys (`BlueprintMapLibrary.Map_Keys` (`self.MovingSpikeTraps`)))
  (for _array_element _keys
    (`/Engine/EditorBlueprintResources/StandardMacros.IsValid` _array_element
      (:`Is Valid`
        (bind _asbp_moving_spike_trap (cast `/Game/Core/Systems/Traps/Dynamic/BP_MovingSpikeTrap` (`ChildActorComponent.ChildActor` _array_element)))
        (set `/Game/Core/Systems/Traps/Dynamic/BP_MovingSpikeTrap.Spline` (`BlueprintMapLibrary.Map_Find` (`self.MovingSpikeTraps`) _array_element) _asbp_moving_spike_trap)))))

(fn `UserConstructionScript`)