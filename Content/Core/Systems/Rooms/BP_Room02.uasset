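; BP_Room02 is a room Blueprint with five moving spike traps and randomized content.
; On BeginPlay, after the parent's logic, it maps each trap to its own path component, starts the traps moving and randomizes the room content.
; An overlap on the entered-room trigger forwards the overlapping actor to the player-entry handler.
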(event `self.ReceiveBeginPlay`
  ;[0 0 0] Begin Play
  (`parent.ReceiveBeginPlay`)
  (set `self.MovingSpikeTraps` (`|MakeMap` (`self.BP_MovingSpikeTrap1`) (`self.SC_TrapPath1`) (`self.BP_MovingSpikeTrap2`) (`self.SC_TrapPath2`) (`self.BP_MovingSpikeTrap3`) (`self.SC_TrapPath3`) (`self.BP_MovingSpikeTrap4`) (`self.SC_TrapPath4`) (`self.BP_MovingSpikeTrap5`) (`self.SC_TrapPath5`)))
  (`self.RunMovingSpikeTraps`)
  (`self.RandomizeContent`))

(event `self.SM_TB_EnteredRoom.OnComponentBeginOverlap`
  (params (OverlappedComponent :type "PrimitiveComponent Object Reference") (OtherActor :type "Actor Object Reference") (OtherComp :type "PrimitiveComponent Object Reference") (OtherBodyIndex :type Integer) (bFromSweep :type Boolean) (SweepResult :type "HitResult Structure (by ref)"))
  ;[0 0 0] Player Enter Room
  (`self.On Player Enter Room` OtherActor))

(fn `UserConstructionScript`)