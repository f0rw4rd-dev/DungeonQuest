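; BP_Sword is a melee weapon Blueprint that destroys certain actors it touches while the player is attacking.
; On BeginPlay it casts player 0's character to BP_CabbageSeller_Character and caches it to read the Attack flag.
; When its Capsule begins an overlap during an attack, it destroys the other actor outright if that actor's class is in ActorsCanBeDestroyed, with no damage step.
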(event `self.ReceiveBeginPlay`
  ;[0 0 0] Begin Play
  (bind _asbp_cabbage_seller_character (cast `/Game/Core/Characters/CabbageSeller/BP_CabbageSeller_Character` (`GameplayStatics.GetPlayerCharacter` 0)))
  (set `self.Character` _asbp_cabbage_seller_character))

(event `self.Capsule.OnComponentBeginOverlap`
  (params (OverlappedComponent :type "PrimitiveComponent Object Reference") (OtherActor :type "Actor Object Reference") (OtherComp :type "PrimitiveComponent Object Reference") (OtherBodyIndex :type Integer) (bFromSweep :type Boolean) (SweepResult :type "HitResult Structure (by ref)"))
  ;[0 0 0] Destroy actors
  (if (`/Game/Core/Characters/CabbageSeller/BP_CabbageSeller_Character.bAttack` (`self.Character`))
    (`/Engine/EditorBlueprintResources/StandardMacros.IsValid` OtherActor
      (:`Is Valid`
        (if (`BlueprintSetLibrary.Set_Contains` (`self.ActorsCanBeDestroyed`) (`GameplayStatics.GetObjectClass` OtherActor))
          (`self.K2_DestroyActor` OtherActor))))))

(fn `UserConstructionScript`)