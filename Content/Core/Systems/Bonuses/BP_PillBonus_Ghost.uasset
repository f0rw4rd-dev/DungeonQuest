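; Ghost pill bonus that temporarily lets the cabbage seller character ignore static traps when picked up.
; Overlap calls Consume, which requires no active bonus on the character and a room, either passed in or taken from the parent actor.
; A DoOnce then hides the pill, sets the bonus and trap-immunity flags, waits the room's bonus duration, clears them and destroys the actor.
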(event `self.ReceiveActorBeginOverlap`
  (params (OtherActor :type "Actor Object Reference"))
  ;[0 0 0] Actor Begin Overlap
  (`parent.ReceiveActorBeginOverlap` OtherActor)
  (`self.Consume` OtherActor))

(event `self.Consume`
  (params (OtherActor :type "Actor Object Reference") (RoomActor :type "Actor Object Reference"))
  ;[0 0 0] Consume Pill
  (cast `/Game/Core/Characters/CabbageSeller/BP_CabbageSeller_Character` OtherActor)
  (if (not (`/Game/Core/Characters/CabbageSeller/BP_CabbageSeller_Character.bBonusEffect` (`self.Character`)))
    (bind _asbp_room (cast `/Game/Core/Systems/Rooms/BP_Room` (select `bool` (`KismetSystemLibrary.IsValid` RoomActor) :`false` (`self.GetParentActor`) :`true` RoomActor)))
    (`/Engine/EditorBlueprintResources/StandardMacros.DoOnce` false
      (:`Completed`
        (set `/Game/Core/Characters/CabbageSeller/BP_CabbageSeller_Character.bBonusEffect` true (`self.Character`))
        (`SceneComponent.SetVisibility` (`self.Pill`) false false)
        (set `/Game/Core/Characters/CabbageSeller/BP_CabbageSeller_Character.bIgnoreStaticTraps` true (`self.Character`))
        (bind (_roominfo_roomnumber _roominfo_maxrooms _roominfo_bhigherdifficulty _roominfo_difficultyfactor _roominfo_trapspeed _roominfo_bonusduration) (break `/Game/Core/Systems/Rooms/F_RoomInfo` (`/Game/Core/Systems/Rooms/BP_Room.RoomInfo` _asbp_room)))
        (`KismetSystemLibrary.Delay` _roominfo_bonusduration)
        (set `/Game/Core/Characters/CabbageSeller/BP_CabbageSeller_Character.bIgnoreStaticTraps` false (`self.Character`))
        (`self.K2_DestroyActor`)
        (set `/Game/Core/Characters/CabbageSeller/BP_CabbageSeller_Character.bBonusEffect` false (`self.Character`))))))

(fn `UserConstructionScript`
  (`parent.UserConstructionScript`))