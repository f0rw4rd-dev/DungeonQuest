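; A pill pickup that temporarily slows the cabbage seller player character.
; Overlap, or a call to Consume, fires once for that character, hiding the pill and lowering max walk speed.
; Duration comes from the room's bonus setting, using the supplied room or falling back to the parent actor.
; Afterwards it restores a hardcoded walk speed rather than the previous value and destroys itself.
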(event `self.ReceiveActorBeginOverlap`
  (params (OtherActor :type "Actor Object Reference"))
  (`parent.ReceiveActorBeginOverlap` OtherActor)
  (`self.Consume` OtherActor))

(event `self.Consume`
  (params (OtherActor :type "Actor Object Reference") (RoomActor :type "Actor Object Reference"))
  (bind _asbp_cabbage_seller_character (cast `/Game/Core/Characters/CabbageSeller/BP_CabbageSeller_Character` OtherActor))
  (bind _asbp_room (cast `/Game/Core/Systems/Rooms/BP_Room` (select `bool` (`KismetSystemLibrary.IsValid` RoomActor) :`false` (`self.GetParentActor`) :`true` RoomActor)))
  (`/Engine/EditorBlueprintResources/StandardMacros.DoOnce` false
    (:`Completed`
      (`SceneComponent.SetVisibility` (`self.Pill`) false false)
      (bind _charactermovement (`Character.CharacterMovement` _asbp_cabbage_seller_character))
      (set `CharacterMovementComponent.MaxWalkSpeed` 150.0 _charactermovement)
      (bind (_roominfo_roomnumber _roominfo_bhigherdifficulty _roominfo_difficultyfactor _roominfo_trapspeed _roominfo_bonusduration) (break `/Game/Core/Systems/Rooms/F_RoomInfo` (`/Game/Core/Systems/Rooms/BP_Room.RoomInfo` _asbp_room)))
      (`KismetSystemLibrary.Delay` _roominfo_bonusduration)
      (set `CharacterMovementComponent.MaxWalkSpeed` 500.0 _charactermovement)
      (`self.K2_DestroyActor`))))

(fn `UserConstructionScript`
  (`parent.UserConstructionScript`))