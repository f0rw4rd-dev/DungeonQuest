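; Random pill bonus pickup that gives the cabbage seller character one of three effects: ghost, slowed player or slowed dynamic objects.
; On overlap with that character, a one-time gate rolls a random choice and spawns the matching pill bonus at its own transform.
; It immediately calls Consume on the spawned bonus, passing the character and its parent actor as the room, then destroys itself.
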(event `self.ReceiveActorBeginOverlap`
  (params (OtherActor :type "Actor Object Reference"))
  ;[0 0 0] Actor Begin Overlap
  (`parent.ReceiveActorBeginOverlap` OtherActor)
  (`self.Consume` OtherActor))

(event `self.Consume`
  (params (OtherActor :type "Actor Object Reference") (RoomActor :type "Actor Object Reference"))
  (bind _returnvalue (`self.GetTransform`))
  (bind _returnvalue_2 (`self.GetParentActor`))
  ;[0 0 0] Random Selection
  (cast `/Game/Core/Characters/CabbageSeller/BP_CabbageSeller_Character` OtherActor)
  (`/Engine/EditorBlueprintResources/StandardMacros.DoOnce` false
    (:`Completed`
      (switch `int` (`KismetMathLibrary.RandomIntegerInRange` 0 2)
        (:`Default`
          (bind _returnvalue_3 (`|SpawnActorFromClass` "/Game/Core/Systems/Bonuses/BP_PillBonus_SlowDownPlayer.BP_PillBonus_SlowDownPlayer_C" _returnvalue "Undefined" "MultiplyWithRoot" null null :!label _label))
          (`self.Consume` _returnvalue_3 OtherActor _returnvalue_2))
        (:`0`
          (bind _returnvalue_4 (`|SpawnActorFromClass` "/Game/Core/Systems/Bonuses/BP_PillBonus_Ghost.BP_PillBonus_Ghost_C" _returnvalue "Undefined" "MultiplyWithRoot" null null))
          (`self.Consume` _returnvalue_4 OtherActor _returnvalue_2))
        (:`1`
          (bind _returnvalue_5 (`|SpawnActorFromClass` "/Game/Core/Systems/Bonuses/BP_PillBonus_SlowDownDynamicObjects.BP_PillBonus_SlowDownDynamicObjects_C" _returnvalue "Undefined" "MultiplyWithRoot" null null))
          (`self.Consume` _returnvalue_5 OtherActor _returnvalue_2))
        (:`2`
          (goto _label)))
      (`self.K2_DestroyActor`))))

(fn `UserConstructionScript`
  (`parent.UserConstructionScript`))