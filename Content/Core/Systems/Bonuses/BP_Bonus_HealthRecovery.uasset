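; Health recovery bonus pickup with a spinning heart that heals the cabbage seller character on contact.
; A timeline started from Tick through a DoOnce, which resets when it finishes, repeatedly drives the heart's yaw rotation.
; On overlap, it calls the character's Heal and destroys itself, but only if that character's health is below the cap.
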(event `self.ReceiveTick`
  (params (DeltaSeconds :type "Float (single-precision)"))
  ;[0 0 0] Rotate
  (`/Engine/EditorBlueprintResources/StandardMacros.DoOnce` false :!label _label
    (:`Completed`
      (bind (_direction _rotation_z) (`Timeline|Timeline` :!via `PlayFromStart`)
        (:`Update`
          (`SceneComponent.K2_SetRelativeRotation` (`self.Heart`) (`KismetMathLibrary.MakeRotator` 0.0 0.0 _rotation_z) false false))
        (:`Finished`
          (goto _label :!via `Reset`))))))

(event `self.Heart.OnComponentBeginOverlap`
  (params (OverlappedComponent :type "PrimitiveComponent Object Reference") (OtherActor :type "Actor Object Reference") (OtherComp :type "PrimitiveComponent Object Reference") (OtherBodyIndex :type Integer) (bFromSweep :type Boolean) (SweepResult :type "HitResult Structure (by ref)"))
  ;[0 0 0] Heal & Destroy
  (bind _asbp_cabbage_seller_character (cast `/Game/Core/Characters/CabbageSeller/BP_CabbageSeller_Character` OtherActor))
  (if (< (`/Game/Core/Characters/CabbageSeller/BP_CabbageSeller_Character.Health` _asbp_cabbage_seller_character) 100)
    (`/Game/Core/Characters/CabbageSeller/BP_CabbageSeller_Character.Heal` _asbp_cabbage_seller_character 0)
    (`self.K2_DestroyActor`)))

(fn `UserConstructionScript`)