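; A pill bonus pickup that temporarily slows a room's moving spike traps when the cabbage seller character consumes it.
; Consume fires on overlap or direct call, finds the BP_Room from a passed actor or its parent actor, and runs once.
; It hides the pill, halves the movement and spike rotation timeline play rates on each trap, restores them after five seconds, then destroys itself.
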(event `self.ReceiveActorBeginOverlap`
  (params (OtherActor :type "Actor Object Reference"))
  (`parent.ReceiveActorBeginOverlap` OtherActor)
  (`self.Consume` OtherActor))

(event `self.Consume`
  (params (OtherActor :type "Actor Object Reference") (RoomActor :type "Actor Object Reference"))
  (cast `/Game/Core/Characters/CabbageSeller/BP_CabbageSeller_Character` OtherActor)
  (bind _asbp_room (cast `/Game/Core/Systems/Rooms/BP_Room` (select `bool` (`KismetSystemLibrary.IsValid` RoomActor) :`false` (`self.GetParentActor`) :`true` RoomActor)))
  (`/Engine/EditorBlueprintResources/StandardMacros.DoOnce` false
    (:`Completed`
      (`SceneComponent.SetVisibility` (`self.Pill`) false false)
      (bind _keys (`BlueprintMapLibrary.Map_Keys` (`/Game/Core/Systems/Rooms/BP_Room.MovingSpikeTraps` _asbp_room)))
      (for _array_element _keys
        (bind _asbp_moving_spike_trap (cast `/Game/Core/Systems/Traps/Dynamic/BP_MovingSpikeTrap` (`ChildActorComponent.ChildActor` _array_element)))
        (`TimelineComponent.SetPlayRate` (`/Game/Core/Systems/Traps/Dynamic/BP_MovingSpikeTrap.MovingTimeline` _asbp_moving_spike_trap) 0.5)
        (`TimelineComponent.SetPlayRate` (`/Game/Core/Systems/Traps/Dynamic/BP_MovingSpikeTrap.RotateSpikesTimeline` _asbp_moving_spike_trap) 0.5))
      (`KismetSystemLibrary.Delay` 5.0)
      (for _array_element_2 _keys
        (bind _asbp_moving_spike_trap_2 (cast `/Game/Core/Systems/Traps/Dynamic/BP_MovingSpikeTrap` (`ChildActorComponent.ChildActor` _array_element_2)))
        (`TimelineComponent.SetPlayRate` (`/Game/Core/Systems/Traps/Dynamic/BP_MovingSpikeTrap.MovingTimeline` _asbp_moving_spike_trap_2) 1.0)
        (`TimelineComponent.SetPlayRate` (`/Game/Core/Systems/Traps/Dynamic/BP_MovingSpikeTrap.RotateSpikesTimeline` _asbp_moving_spike_trap_2) 1.0))
      (`self.K2_DestroyActor`))))

(fn `UserConstructionScript`
  (`parent.UserConstructionScript`))