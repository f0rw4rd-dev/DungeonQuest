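; BP_MovingSpikeTrap is a hazard that spins while moving along a spline and hurts BP_CabbageSeller_Character on hit.
; A timeline moves it by spline distance in world XY, keeping its current height.
; A second timeline yaws the spike component, restarted on completion through a Tick-driven DoOnce.
; When its parent actor is a BP_Room, both timelines take their play rate from that room's TrapSpeed.
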(event `self.ReceiveBeginPlay`
  ;[0 0 0] Begin play
  (`self.StartMoving`)
  (bind _asbp_room (cast `/Game/Core/Systems/Rooms/BP_Room` (`self.GetParentActor`)))
  (bind (_roominfo_roomnumber _roominfo_bhigherdifficulty _roominfo_difficultyfactor _roominfo_trapspeed) (break `/Game/Core/Systems/Rooms/F_RoomInfo` (`/Game/Core/Systems/Rooms/BP_Room.RoomInfo` _asbp_room)))
  (`TimelineComponent.SetPlayRate` (`self.MovingTimeline`) _roominfo_trapspeed)
  (`TimelineComponent.SetPlayRate` (`self.RotateSpikesTimeline`) _roominfo_trapspeed))

(event `self.ReceiveTick`
  (params (DeltaSeconds :type "Float (single-precision)"))
  ;[0 0 0] Rotate spikes
  (`/Engine/EditorBlueprintResources/StandardMacros.DoOnce` false :!label _label
    (:`Completed`
      (bind (_direction _rotation_z) (`Timeline|RotateSpikesTimeline` :!via `PlayFromStart`)
        (:`Update`
          (`SceneComponent.K2_SetRelativeRotation` (`self.MovingSpikeTrap`) (`KismetMathLibrary.MakeRotator` 0.0 0.0 _rotation_z) false false))
        (:`Finished`
          (goto _label :!via `Reset`))))))

(event `self.MovingSpikeTrap.OnComponentHit`
  (params (HitComponent :type "PrimitiveComponent Object Reference") (OtherActor :type "Actor Object Reference") (OtherComp :type "PrimitiveComponent Object Reference") (NormalImpulse :type "Vector Structure") (Hit :type "HitResult Structure (by ref)"))
  ;[0 0 0] Cause damage
  (bind _asbp_cabbage_seller_character (cast `/Game/Core/Characters/CabbageSeller/BP_CabbageSeller_Character` OtherActor))
  (`/Game/Core/Characters/CabbageSeller/BP_CabbageSeller_Character.Hurt` _asbp_cabbage_seller_character 0))

(event `StartMoving`
  (bind (_returnvalue_x _returnvalue_y _returnvalue_z) (`KismetMathLibrary.BreakVector` (`self.K2_GetActorLocation`)))
  ;[0 0 0] Start moving
  (bind (_direction _alpha) (`Timeline|MovingTimeline`)
    (:`Update`
      (`/Engine/EditorBlueprintResources/StandardMacros.IsValid` (`self.Spline`)
        (:`Is Valid`
          (bind (_returnvalue_x_2 _returnvalue_y_2) (`KismetMathLibrary.BreakVector` (`SplineComponent.GetLocationAtDistanceAlongSpline` (`self.Spline`) (`KismetMathLibrary.Lerp` 0.0 (`SplineComponent.GetSplineLength` (`self.Spline`)) _alpha) "World")))
          (`self.K2_SetActorLocation` (`KismetMathLibrary.MakeVector` _returnvalue_x_2 _returnvalue_y_2 _returnvalue_z)))))))

(fn `UserConstructionScript`)